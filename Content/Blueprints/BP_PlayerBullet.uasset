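; BP_PlayerBullet is a player projectile that damages enemies on overlap.
; Tick counts BulletLifeSpan down and destroys the bullet when it runs out.
; On overlapping an Enemy it subtracts a fixed amount directly from that enemy's Health, then destroys itself; other actors are ignored.
; An AddForce call on BulletObject is left unconnected, so this graph does not propel the bullet.
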(event EventBeginPlay)

(event EventTick
  (params (DeltaSeconds :type Float%20%28single-precision%29))
  (bind _output_get (Variables|Default|SetbulletLifeSpan (- (Variables|Default|GetbulletLifeSpan) DeltaSeconds)))
  (if (<= _output_get 0.0)
    (Actor|DestroyActor)))

(event Collision|EventActorBeginOverlap
  (params (OtherActor :type Actor%20Object%20Reference))
  ;[1 1 1] Deal damage to enemy
  (bind _asenemy (Utilities|Casting|CastToEnemy OtherActor))
  (if true
    (Variables|/Game/Blueprints/Enemy.Enemy_C|SetHealth _asenemy (- (Variables|/Game/Blueprints/Enemy.Enemy_C|GetHealth _asenemy) 10))
    (Actor|DestroyActor)))

(fn ConstructionScript)