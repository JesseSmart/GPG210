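; Enemy character that chases the player, deals melee damage and reports its death to the wave manager.
; Tick issues AI MoveTo toward the player, updates the health bar widget, turns the enemy to face them and destroys it at zero health, decrementing BP_WaveManager's spawn count.
; Overlapping the player starts attacking: Tick calls a Delay-throttled Attack that damages the player and refreshes the main UI while in range.
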(event Custom|Attack
  (bind _characterref (Variables|Default|GetCharacterRef))
  ;[1 1 1] Attacking
  (Utilities|FlowControl|Delay 1.0)
  (if (<= (Transformation|GetDistanceTo (Variables|Default|GetCharacterRef)) 1e+02)
    (Variables|/Game/Blueprints/PlayerCharacter.PlayerCharacter_C|SetHealth _characterref (- (Variables|/Game/Blueprints/PlayerCharacter.PlayerCharacter_C|GetHealth _characterref) 10))
    (bind _foundwidgets (Widget|GetAllWidgetsOfClass "/Game/Scenes/Blueprints/BP_MainUI.BP_MainUI_C" true))
    (Default|UpdateHealthBar (Utilities|Array|Get(acopy) _foundwidgets))
    (else
      (Variables|Default|SetAttacking false))))

(event EventTick
  (params (DeltaSeconds :type Float%20%28single-precision%29))
  (bind _widget (Variables|Default|GetWidget))
  ;[1 1 1] Update
  ;;[1 1 1] Move To Player
  (if (Variables|Default|GetAttacking)
    (CallFunction|Attack))
  (bind _outactors (Actor|GetAllActorsOfClass "/Game/Blueprints/PlayerCharacter.PlayerCharacter_C"))
  (AI|AIMoveTo self "0, 0, 0" (Utilities|Array|Get(acopy) _outactors) 5.0 false
    (:then
      ;;[1 1 1] Set Health Bar
      (bind _aswt_enemy_health_bar (Utilities|Casting|CastToWT_EnemyHealthBar (UserInterface|GetUserWidgetObject (Variables|Default|GetWidget))))
      (Progress|SetPercent (Variables|/Game/Widget/WT_EnemyHealthBar.WT_EnemyHealthBar_C|GetProgressBar_265 _aswt_enemy_health_bar) (/ (Math|Conversions|ToFloat(Integer) (Variables|Default|GetHealth)) 1e+02))
      (bind _outactors_2 (Actor|GetAllActorsOfClass "/Game/Blueprints/PlayerCharacter.PlayerCharacter_C"))
      (Transformation|SetActorRotation (Components|GetOwner _widget) (Math|Rotator|FindLookatRotation (Transformation|GetWorldLocation _widget) (Transformation|GetActorLocation (Utilities|Array|Get(acopy) _outactors_2))))
      ;;[1 1 1] Check Health | Die
      (if (<= (Variables|Default|GetHealth) 0)
        (Actor|DestroyActor)
        (bind _outactors_3 (Actor|GetAllActorsOfClass "/Game/Scenes/Blueprints/BP_WaveManager.BP_WaveManager_C"))
        (bind _result (Math|Integer|DecrementInt (Variables|/Game/Scenes/Blueprints/BP_WaveManager.BP_WaveManager_C|GetspawnedCount (Utilities|Array|Get(acopy) _outactors_3)))
          (:%20%20
            (Variables|/Game/Scenes/Blueprints/BP_WaveManager.BP_WaveManager_C|SetspawnedCount (Utilities|Array|Get(acopy) _outactors_3) _result)
            (Default|CheckEnemyCount (Utilities|Array|Get(acopy) _outactors_3))))))))

(event EventBeginPlay
  ;[1 1 1] Initialise Speed
  (Variables|/Script/Engine.CharacterMovementComponent|SetMaxWalkSpeed (Variables|Character|GetCharacterMovement) 5e+02))

(event Collision|EventActorBeginOverlap
  (params (OtherActor :type Actor%20Object%20Reference))
  ;[1 1 1] On Collision
  (bind _asplayer_character (Utilities|Casting|CastToPlayerCharacter OtherActor))
  (if true
    (Variables|Default|SetCharacterRef _asplayer_character)
    (Variables|Default|SetAttacking true)))

(fn ConstructionScript)