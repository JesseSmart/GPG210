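; BP_EndOfLevel is an end-of-level trigger that shuts off enemy spawning and opens the exit once the remaining spawns are cleared.
; When a PlayerCharacter overlaps it, it destroys every BP_SpawnerController and sets Endgame inside that loop.
; While Endgame is set, Tick polls the first BP_WaveManager and, whenever SpawnedCount is zero, destroys the first actor tagged "enddoor".
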(event EventBeginPlay)

(event Collision|EventActorBeginOverlap
  (params (OtherActor :type Actor%20Object%20Reference))
  (Utilities|Casting|CastToPlayerCharacter OtherActor)
  (bind _outactors (Actor|GetAllActorsOfClass "/Game/Scenes/Blueprints/BP_SpawnerController.BP_SpawnerController_C"))
  (for _array_element _outactors
    (Actor|DestroyActor _array_element)
    (Variables|Default|Setendgame true)))

(event EventTick
  (params (DeltaSeconds :type Float%20%28single-precision%29))
  (if (Variables|Default|Getendgame)
    (bind _outactors (Actor|GetAllActorsOfClass "/Game/Scenes/Blueprints/BP_WaveManager.BP_WaveManager_C"))
    (if (== (Variables|/Game/Scenes/Blueprints/BP_WaveManager.BP_WaveManager_C|GetspawnedCount (Utilities|Array|Get(acopy) _outactors)) 0)
      (bind _outactors_2 (Actor|GetAllActorswithTag "enddoor"))
      (Actor|DestroyActor (Utilities|Array|Get(acopy) _outactors_2)))))

(fn ConstructionScript)