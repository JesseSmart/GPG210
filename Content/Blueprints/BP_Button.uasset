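; BP_Button is a pressure-button actor that removes a tagged set of actors when a player holding the key steps on it.
; On overlap, it casts to PlayerCharacter, checks HasKey, then swaps the cylinder's material to a pressed look.
; It then gathers all actors with a hard-coded tag, prints their count and destroys them in a loop, with no direct references to the targets.
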(event EventBeginPlay)

(event Collision|EventActorBeginOverlap
  (params (OtherActor :type Actor%20Object%20Reference))
  (bind _asplayer_character (Utilities|Casting|CastToPlayerCharacter OtherActor))
  (if (Variables|/Game/Blueprints/PlayerCharacter.PlayerCharacter_C|GethasKey _asplayer_character)
    (Rendering|Material|SetMaterial (Variables|Default|GetCylinder) 0 "/Game/Materials/MTI_ButtonPressed.MTI_ButtonPressed")
    (bind _outactors (Actor|GetAllActorswithTag "bitchboi"))
    (Development|PrintString (Utilities|String|ToString(Integer) (Utilities|Array|Length _outactors)))
    (for _index (range 0 (Utilities|Array|Length _outactors))
      (Actor|DestroyActor (Utilities|Array|Get(acopy) _outactors _index)))))

(event EventTick
  (params (DeltaSeconds :type Float%20%28single-precision%29)))

(fn ConstructionScript)