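; BP_Enemy is an enemy Blueprint whose Box component homes in on the player character.
; BeginPlay caches all ThirdPersonCharacter actors, and Tick targets the first one.
; Each frame, the Box's world location lerps toward that character's capsule using DeltaSeconds as alpha, giving an eased follow without sweep collision.
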(event EventTick
  (params (DeltaSeconds :type Float%20%28single-precision%29))
  (bind _box (Variables|Default|GetBox))
  (bind _output_get (Variables|Default|SetPlayer (Utilities|Array|Get(acopy) (Variables|Default|GetThePlayer))))
  (Transformation|SetWorldLocation _box (Math|Vector|Lerp(Vector) (Transformation|GetWorldLocation _box) (Transformation|GetWorldLocation (Variables|/Script/Engine.Character|GetCapsuleComponent _output_get)) DeltaSeconds) false false))

(event EventBeginPlay
  (bind _outactors (Actor|GetAllActorsOfClass "/Game/ThirdPersonBP/Blueprints/ThirdPersonCharacter.ThirdPersonCharacter_C"))
  (Variables|Default|SetThePlayer _outactors))

(fn ConstructionScript)