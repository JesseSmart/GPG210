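; BP_WaveManager is a wave manager that advances enemy waves through the level's BP_SpawnerController actors.
; On BeginPlay it registers itself as WaveController on every spawner.
; CheckEnemyCount increments the wave when SpawnedCount is zero, updates MainUI, then either tells all spawners to spawn a fixed batch or prints "finish" at WaveMax, unless waves are unlimited.
; The temporary overlap trigger for that check is disconnected.
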(event EventBeginPlay
  (bind _outactors (Actor|GetAllActorsOfClass "/Game/Scenes/Blueprints/BP_SpawnerController.BP_SpawnerController_C"))
  (bind _output_get (Variables|Default|SetallSpawners _outactors))
  (for _array_element _output_get
    (Variables|/Game/Scenes/Blueprints/BP_SpawnerController.BP_SpawnerController_C|SetwaveController _array_element self)))

(event Collision|EventActorBeginOverlap
  (params (OtherActor :type Actor%20Object%20Reference))
  ;[1 1 1] Temporary. Run check on collision
)

(event EventTick
  (params (DeltaSeconds :type Float%20%28single-precision%29)))

(fn ConstructionScript)

(fn CheckEnemyCount
  ;[1 1 1] Check for number of enemies
  (if (== (Variables|Default|GetspawnedCount) 0)
    ;[1 1 1] Increment wave number if there are no enemies
    (bind _result (Math|Integer|IncrementInt (Variables|Default|GetwaveNumber))
      (:%20%20
        (Variables|Default|SetwaveNumber _result)
        (Default|UpdateWaveCounter (Variables|Default|GetmainUI))
        ;[1 1 1] Control when to spawn waves or progress game
        (if (Variables|Default|GetisUnlimitedWaves)
          (CallFunction|SpawnNewWave :!label _label)
          (elif (< (Variables|Default|GetwaveNumber) (Variables|Default|GetwaveMax))
            (goto _label)
            (else
              (Development|PrintString "finish"))))))))

(fn SpawnNewWave
  (bind _outactors (Actor|GetAllActorsOfClass "/Game/Scenes/Blueprints/BP_SpawnerController.BP_SpawnerController_C"))
  (for _array_element _outactors
    (Variables|/Game/Scenes/Blueprints/BP_SpawnerController.BP_SpawnerController_C|SetnumberToSpawn _array_element 5)
    (Default|ToSpawn _array_element)))