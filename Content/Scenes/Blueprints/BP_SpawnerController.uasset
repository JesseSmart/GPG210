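; Enemy spawner actor that places AI enemies at randomized offsets around its Cube and updates the WaveController's spawned and remaining counts.
; ToSpawn spawns a wave through delayed for and while macros, one enemy at a time, stalling while the spawned count exceeds a cap.
; Separately, Tick watches the first PlayerCharacter for HasKey; with TriggerSpawner set, it spawns one enemy and destroys itself.
; SpawnEnemies is empty, and several older spawn chains are left disconnected.
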(event Custom|ToSpawn
  (Utilities|ForLoopwithDelay 0 (Variables|/Game/Scenes/Blueprints/BP_WaveManager.BP_WaveManager_C|GetNumberToSpawn (Variables|Default|GetwaveController)) :!label _label
    (:loopBody
      (Utilities|WhilewithDelay (> (Variables|/Game/Scenes/Blueprints/BP_WaveManager.BP_WaveManager_C|GetspawnedCount (Variables|Default|GetwaveController)) 25) :!label _label_2
        (:completed
          (if (> (Variables|/Game/Scenes/Blueprints/BP_WaveManager.BP_WaveManager_C|GetNumberToSpawn (Variables|Default|GetwaveController)) 0)
            (CallFunction|SpawninEnemy)))
        (:delayOut
          (Utilities|FlowControl|Delay 2.5)
          (goto _label_2 delayIn))))
    (:delayOut
      (Utilities|FlowControl|Delay 1.0)
      (goto _label delayIn))))

(event EventBeginPlay)

(event Collision|EventActorBeginOverlap
  (params (OtherActor :type Actor%20Object%20Reference)))

(event EventTick
  (params (DeltaSeconds :type Float%20%28single-precision%29))
  (bind _outactors (Actor|GetAllActorsOfClass "/Game/Blueprints/PlayerCharacter.PlayerCharacter_C"))
  (if (Variables|/Game/Blueprints/PlayerCharacter.PlayerCharacter_C|GethasKey (Utilities|Array|Get(acopy) _outactors))
    (if (Variables|Default|GetTriggerSpawner)
      (CallFunction|SpawninEnemy)
      (Actor|DestroyActor))))

(fn ConstructionScript)

(fn SpawnEnemies)

(fn SpawninEnemy
  (bind _cube (Variables|Default|GetCube))
  (bind _wavecontroller (Variables|Default|GetwaveController))
  (bind _wavecontroller_2 (Variables|Default|GetwaveController))
  (bind _returnvalue (Transformation|GetWorldTransform _cube))
  (bind _output_get (Variables|Default|SetspawnArea (Math|Transform|MakeTransform (Math|Vector|MakeVector (+ (.x (.location _returnvalue)) (* (Math|Trig|Sin(Degrees) (Math|Random|RandomFloatinRange 0.0 3.6e+02)) 2.5e+02)) (+ (.y (.location _returnvalue)) (* (Math|Trig|Cos(Degrees) (Math|Random|RandomFloatinRange 0.0 3.6e+02)) 2.5e+02)) (.z (.location _returnvalue))) "0, 0, 0" "1,1,1")))
  ;[1 1 1] credit to josh knight, the greatest spaghetti coder
  (AI|SpawnAIFromClass "/Game/Blueprints/Enemy.Enemy_C" 0 (Math|Transform|TransformLocation _output_get "0, 0, 0") "0, 0, 0" false)
  (bind _result (Math|Integer|IncrementInt (Variables|/Game/Scenes/Blueprints/BP_WaveManager.BP_WaveManager_C|GetspawnedCount _wavecontroller_2))
    (:%20%20
      (Variables|/Game/Scenes/Blueprints/BP_WaveManager.BP_WaveManager_C|SetspawnedCount _wavecontroller_2 _result)
      (bind _result_2 (Math|Integer|DecrementInt (Variables|/Game/Scenes/Blueprints/BP_WaveManager.BP_WaveManager_C|GetNumberToSpawn _wavecontroller))
        (:%20%20
          (Variables|/Game/Scenes/Blueprints/BP_WaveManager.BP_WaveManager_C|SetNumberToSpawn _wavecontroller _result_2))))))